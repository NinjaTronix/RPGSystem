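; BP_LevelTransitionCrytals is a trigger that moves the player to another level in exchange for a required crystal.
; On overlap it casts to CH_MyCharacter, saves the game, then searches the character's OwnedCrytals for RequiredCrystalType.
; A match is removed from that array, the remaining crystals are copied to OwnedCrystalsGameInstance, and the level named by LevelName opens.
; The save runs on every character overlap, before the crystal check and removal.
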(event `self.Overlap.OnComponentBeginOverlap`
  (params (OverlappedComponent :type "PrimitiveComponent Object Reference") (OtherActor :type "Actor Object Reference") (OtherComp :type "PrimitiveComponent Object Reference") (OtherBodyIndex :type Integer) (bFromSweep :type Boolean) (SweepResult :type "HitResult Structure (by ref)"))
  (bind _asch_my_character (cast `/Game/Characters/Player/CH_MyCharacter` OtherActor))
  (`/Game/Characters/Player/CH_MyCharacter.SaveGame` _asch_my_character)
  (bind _ownedcrytals (`/Game/Characters/Player/CH_MyCharacter.OwnedCrytals` _asch_my_character))
  (for (_array_element _array_index) _ownedcrytals
    (if (`|EnumEquality` _array_element (`self.RequiredCrystalType`))
      (`KismetArrayLibrary.Array_Remove` _ownedcrytals _array_index)
      (bind _asowned_crystals_game_instance (cast `/Game/DoorsAndCrystals/OwnedCrystalsGameInstance` (`GameplayStatics.GetGameInstance`)))
      (set `/Game/DoorsAndCrystals/OwnedCrystalsGameInstance.PlayerCrystals` _ownedcrytals _asowned_crystals_game_instance)
      (`GameplayStatics.OpenLevel` (`self.LevelName`)))))

(fn `UserConstructionScript`)