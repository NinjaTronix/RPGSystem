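; BP_OpeningDoor is a key-gated door that swings open when a CH_MyCharacter with enough keys enters its overlap volume.
; Entry deducts the required keys, even if the door is already open, or prints a red warning when keys are short.
; The DoorRotation timeline drives yaw from the starting rotation, and leaving reverses it after a retriggerable two-second delay.
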(event `self.ReceiveBeginPlay`
  (set `self.InitialRotation` (`self.K2_GetActorRotation`)))

(event `self.Overlap.OnComponentBeginOverlap`
  (params (OverlappedComponent :type "PrimitiveComponent Object Reference") (OtherActor :type "Actor Object Reference") (OtherComp :type "PrimitiveComponent Object Reference") (OtherBodyIndex :type Integer) (bFromSweep :type Boolean) (SweepResult :type "HitResult Structure (by ref)"))
  (bind _requirednumberofkeys (`self.RequiredNumberOfKeys`))
  (bind _asch_my_character (cast `/Game/Characters/Player/CH_MyCharacter` OtherActor))
  (bind _numberofkeys (`/Game/Characters/Player/CH_MyCharacter.NumberOfKeys` _asch_my_character))
  (if (>= _numberofkeys _requirednumberofkeys)
    (set `/Game/Characters/Player/CH_MyCharacter.NumberOfKeys` (- _numberofkeys _requirednumberofkeys) _asch_my_character)
    (if (not (`self.IsDoorOpen`))
      (set `self.IsDoorOpen` true)
      (bind (_direction _rotation) (`Timeline|DoorRotation` :!label _label)
        (:`Update`
          (`self.K2_SetActorRelativeRotation` (`KismetMathLibrary.MakeRotator` 0.0 0.0 (+ _rotation (.yaw (`self.InitialRotation`))))))))
    (else
      (`KismetSystemLibrary.PrintString` "You don't have enough keys" true true (struct :`R` 1.0 :`A` 1.0)))))

(event `self.Overlap.OnComponentEndOverlap`
  (params (OverlappedComponent :type "PrimitiveComponent Object Reference") (OtherActor :type "Actor Object Reference") (OtherComp :type "PrimitiveComponent Object Reference") (OtherBodyIndex :type Integer))
  (cast `/Game/Characters/Player/CH_MyCharacter` OtherActor)
  (`KismetSystemLibrary.RetriggerableDelay` 2.0)
  (set `self.IsDoorOpen` false)
  (goto _label :!via `Reverse`))

(fn `UserConstructionScript`)