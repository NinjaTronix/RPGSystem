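; Level transition trigger that lets CH_MyCharacter travel to a named level in exchange for keys.
; On overlap it compares the character's key count to RequiredNumberOfKeys, deducts that amount, saves the game and opens LevelName.
; When keys are required it also removes exactly two inventory entries, whatever the required number, and refreshes the inventory.
; Without enough keys it prints a red warning.
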(event `self.Overlap.OnComponentBeginOverlap`
  (params (OverlappedComponent :type "PrimitiveComponent Object Reference") (OtherActor :type "Actor Object Reference") (OtherComp :type "PrimitiveComponent Object Reference") (OtherBodyIndex :type Integer) (bFromSweep :type Boolean) (SweepResult :type "HitResult Structure (by ref)"))
  (bind _requirednumberofkeys (`self.RequiredNumberOfKeys`))
  (bind _asch_my_character (cast `/Game/Characters/Player/CH_MyCharacter` OtherActor))
  (bind _numberofkeys (`/Game/Characters/Player/CH_MyCharacter.NumberOfKeys` _asch_my_character))
  (if (>= _numberofkeys _requirednumberofkeys)
    (set `/Game/Characters/Player/CH_MyCharacter.NumberOfKeys` (- _numberofkeys _requirednumberofkeys) _asch_my_character)
    (if (> (`self.RequiredNumberOfKeys`) 0)
      (`/Game/Characters/Player/CH_MyCharacter.RemoveFromInventory` :`self` _asch_my_character)
      (`/Game/Characters/Player/CH_MyCharacter.RemoveFromInventory` :`self` _asch_my_character)
      (`/Game/Characters/Player/CH_MyCharacter.RefreshInventory` _asch_my_character)
      (`/Game/Characters/Player/CH_MyCharacter.SaveGame` _asch_my_character)
      (`GameplayStatics.OpenLevel` (`self.LevelName`))
      (else
        (`/Game/Characters/Player/CH_MyCharacter.SaveGame` _asch_my_character)
        (`GameplayStatics.OpenLevel` (`self.LevelName`))))
    (else
      (`KismetSystemLibrary.PrintString` "You don't have enough keys" true true (struct :`R` 1.0 :`A` 1.0)))))

(fn `UserConstructionScript`)