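; BP_HeathItem_3 is a health pickup that heals a CH_MyCharacter overlapping it.
; If health is below a hard-coded 100, it adds PlusHP, clamped to MaxHealth, then plays a sound at world origin, spawns sparks at the item and destroys itself.
; It then passes the new health to player 0's CallUpdateHealth.
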(event `self.Overlap.OnComponentBeginOverlap`
  (params (OverlappedComponent :type "PrimitiveComponent Object Reference") (OtherActor :type "Actor Object Reference") (OtherComp :type "PrimitiveComponent Object Reference") (OtherBodyIndex :type Integer) (bFromSweep :type Boolean) (SweepResult :type "HitResult Structure (by ref)"))
  (bind _asch_my_character (cast `/Game/Characters/Player/CH_MyCharacter` OtherActor))
  (if (< (`/Game/Characters/Player/CH_MyCharacter.CurrentHealth` _asch_my_character) 100.0)
    (bind _output_get (set `/Game/Characters/Player/CH_MyCharacter.CurrentHealth` (+ (`/Game/Characters/Player/CH_MyCharacter.CurrentHealth` _asch_my_character) (`self.PlusHP`)) _asch_my_character))
    (bind _maxhealth (`/Game/Characters/Player/CH_MyCharacter.MaxHealth` _asch_my_character))
    (if (> _output_get _maxhealth)
      (bind _output_get_2 (set `/Game/Characters/Player/CH_MyCharacter.CurrentHealth` _maxhealth _asch_my_character)))
    (`GameplayStatics.PlaySoundAtLocation` "/Game/Audio/SFX/healspell1.healspell1" (0.0 0.0 0.0) (struct) 1.0 1.0 0.0 null null null)
    (`GameplayStatics.SpawnEmitterAtLocation` "/Game/StarterContent/Particles/P_SparksHealth.P_SparksHealth" (`SceneComponent.K2_GetComponentLocation` (`self.HealthItem`)))
    (`self.K2_DestroyActor`)
    (bind _asch_my_character_2 (cast `/Game/Characters/Player/CH_MyCharacter` (`GameplayStatics.GetPlayerCharacter` 0)))
    (`/Game/Characters/Player/CH_MyCharacter.UpdateHealth` _asch_my_character_2 _output_get_2)))

(fn `UserConstructionScript`)