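; BP_BaseItem is a base pickup item that moves into the interacting instigator's inventory.
; On interaction it checks the instigator for inventory space, sends its ItemInfo struct through PickupMessage, then destroys itself; without space, nothing happens.
; The construction script rebuilds ItemInfo with the actor's own class, keeping the other fields, so the struct records which class the item came from.
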(event `/Game/Interactables/BPI_interact.Interaction`
  (params (Instigator :type "/Game/Characters/Player/CH_MyCharacter Object Reference"))
  (if (`/Game/Characters/Player/CH_MyCharacter.HasSpaceInInventory` Instigator)
    (message `/Game/Interactables/BPI_interact.Pickup` Instigator (`self.ItemInfo`))
    (`self.K2_DestroyActor`)))

(fn `UserConstructionScript`
  (bind (_iteminfo_itemtype _iteminfo_itemname _iteminfo_itemimage _iteminfo_itemclass _iteminfo_itemindex _iteminfo_itemslot _iteminfo_itemvalue) (break `/Game/Interactables/FItemInfo` (`self.ItemInfo`)))
  (`parent.UserConstructionScript`)
  (set `self.ItemInfo` (make `/Game/Interactables/FItemInfo` _iteminfo_itemtype _iteminfo_itemname _iteminfo_itemimage (`GameplayStatics.GetObjectClass` self) _iteminfo_itemindex _iteminfo_itemslot _iteminfo_itemvalue)))