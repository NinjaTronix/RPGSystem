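; Kunai projectile interactable that deals damage on overlap and can be picked up to restock the instigator's kunai, up to a cap.
; Interaction increments the instigator's kunai count and destroys the actor.
; The first InteractableArea overlap fires a sphere trace forward from the cached player character, rather than from the projectile.
; A DoOnce with delayed reset limits damage to one hit actor per burst, credited to the player.
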(event `/Game/Interactables/BPI_interact.Interaction`
  (params (Instigator :type "/Game/Characters/Player/CH_MyCharacter Object Reference"))
  (bind _kunai (`/Game/Characters/Player/CH_MyCharacter.Kunai` Instigator))
  ;[1 0 0.0418] used this to fix some errors, but still not sure why it was needed..
  (`/Engine/EditorBlueprintResources/StandardMacros.IsValid` "BP_Kunai_Projectile"
    (:`Is Valid`
      (if (< _kunai 10)
        (set `/Game/Characters/Player/CH_MyCharacter.Kunai` (+ _kunai 1) Instigator)
        (`self.K2_DestroyActor`)))))

(event `self.ReceiveBeginPlay`
  (bind _asch_my_character (cast `/Game/Characters/Player/CH_MyCharacter` (`GameplayStatics.GetPlayerCharacter` 0)))
  (set `self.CharacterReference` _asch_my_character))

(event `self.InteractableArea.OnComponentBeginOverlap`
  (params (OverlappedComponent :type "PrimitiveComponent Object Reference") (OtherActor :type "Actor Object Reference") (OtherComp :type "PrimitiveComponent Object Reference") (OtherBodyIndex :type Integer) (bFromSweep :type Boolean) (SweepResult :type "HitResult Structure (by ref)"))
  (bind _characterreference (`self.CharacterReference`))
  (bind _returnvalue (`self.K2_GetActorLocation` _characterreference))
  (`/Engine/EditorBlueprintResources/StandardMacros.DoOnce` false
    (:`Completed`
      (bind (_outhits _returnvalue_2) (`KismetSystemLibrary.SphereTraceMulti` _returnvalue (+ _returnvalue (* (`self.GetActorForwardVector` _characterreference) (`self.Range`))) 25.0 "TraceTypeQuery2" false (`|MakeArray` _characterreference (`self.NPC Roam`) (`self.NPC Turn`) :!type "Actor Object Reference")))
      (if _returnvalue_2
        (for _array_element _outhits
          (`/Engine/EditorBlueprintResources/StandardMacros.DoOnce` false :!label _label
            (:`Completed`
              (`GameplayStatics.ApplyDamage` (`.HitActor` (`GameplayStatics.BreakHitResult` _array_element)) (`self.Damage`) null (`self.CharacterReference`))
              (`KismetSystemLibrary.Delay` 0.5)
              (goto _label :!via `Reset`))))))))

(fn `UserConstructionScript`
  (`parent.UserConstructionScript`))