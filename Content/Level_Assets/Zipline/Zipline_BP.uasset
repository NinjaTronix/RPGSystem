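; Zipline actor that carries the player along a spline when F is pressed, with input enabled only while the character overlaps the start point.
; The construction script positions start and end points and builds spline mesh segments between spline points.
; A timeline scaled by Playrate sweeps the character along the spline at a fixed downward offset.
; OnZipline clears after a rate-scaled hang-time delay, and a DoOnce blocks retriggering until the timeline finishes.
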(event `self.ReceiveBeginPlay`
  (bind _asch_my_character (cast `/Game/Characters/Player/CH_MyCharacter` (`GameplayStatics.GetPlayerCharacter` 0)))
  (set `self.CharacterRef` _asch_my_character)
  (`TimelineComponent.SetPlayRate` (`self.ZipTime`) (`self.Playrate`)))

(event `self.Startpoint.OnComponentBeginOverlap`
  (params (OverlappedComponent :type "PrimitiveComponent Object Reference") (OtherActor :type "Actor Object Reference") (OtherComp :type "PrimitiveComponent Object Reference") (OtherBodyIndex :type Integer) (bFromSweep :type Boolean) (SweepResult :type "HitResult Structure (by ref)"))
  ;[1 1 1] Toggles Control
  (cast `/Game/Characters/Player/CH_MyCharacter` OtherActor)
  (`self.EnableInput` (`GameplayStatics.GetPlayerController` 0)))

(event `Key|F`
  (params (Key :type "Key Structure"))
  ;[1 1 1] Zipline Movement
  (:`Pressed`
    (`/Engine/EditorBlueprintResources/StandardMacros.DoOnce` false :!label _label
      (:`Completed`
        (bind _asch_my_character (cast `/Game/Characters/Player/CH_MyCharacter` (`GameplayStatics.GetPlayerCharacter` 0)))
        (set `/Game/Characters/Player/CH_MyCharacter.OnZipline?` true _asch_my_character)
        (bind (_direction _movement) (`Timeline|ZipTime` :`NewTime` 0.2 :!via `PlayFromStart`)
          (:`Update`
            (`self.K2_SetActorLocation` (`self.CharacterRef`) (`KismetMathLibrary.MakeVector` (.x (`SplineComponent.GetLocationAtDistanceAlongSpline` (`self.Zipline`) (* (`SplineComponent.GetSplineLength` (`self.Zipline`)) _movement) "World")) (.y (`SplineComponent.GetLocationAtDistanceAlongSpline` (`self.Zipline`) (* (`SplineComponent.GetSplineLength` (`self.Zipline`)) _movement) "World")) (- (.z (`SplineComponent.GetLocationAtDistanceAlongSpline` (`self.Zipline`) (* (`SplineComponent.GetSplineLength` (`self.Zipline`)) _movement) "World")) 140.0)) true false)
            (`KismetSystemLibrary.Delay` (/ (`self.Hangtime`) (`self.Playrate`)))
            (set `/Game/Characters/Player/CH_MyCharacter.OnZipline?` false _asch_my_character))
          (:`Finished`
            (`self.Reset`)))))))

(event `self.Startpoint.OnComponentEndOverlap`
  (params (OverlappedComponent :type "PrimitiveComponent Object Reference") (OtherActor :type "Actor Object Reference") (OtherComp :type "PrimitiveComponent Object Reference") (OtherBodyIndex :type Integer))
  ;[1 1 1] Toggles Control
  (cast `/Game/Characters/Player/CH_MyCharacter` OtherActor)
  (`self.DisableInput` (`GameplayStatics.GetPlayerController` 0)))

(event `Reset`
  ;[1 1 1] Zipline Movement
  (goto _label :!via `Reset`))

(fn `UserConstructionScript`
  (bind _zipline (`self.Zipline`))
  (bind _mesh (`self.Mesh`))
  (bind _returnvalue (`SplineComponent.GetNumberOfSplinePoints` (`self.Zipline`)))
  (for _index (range (+ (- _returnvalue 2) 1))
    ;[1 1 1] Sets Start and End Points
    (`SceneComponent.K2_SetRelativeLocation` (`self.Startpoint`) (`SplineComponent.GetLocationAndTangentAtSplinePoint` _zipline (`|GetArrayItem` (`|MakeArray` _returnvalue) _returnvalue) "Local") false false)
    (`SceneComponent.K2_SetRelativeLocation` (`self.EndPoint`) (`SplineComponent.GetLocationAndTangentAtSplinePoint` _zipline (`|GetArrayItem` (`|MakeArray` _returnvalue)) "Local") false false)
    (bind _returnvalue_2 (`AddComponent|NODE_AddSplineMeshComponent-0`))
    (`SceneComponent.K2_AttachToComponent` (`self.DefaultSceneRoot`) _returnvalue_2 "None" "KeepRelative" "KeepRelative" "KeepRelative" true)
    (bind (_location _tangent) (`SplineComponent.GetLocationAndTangentAtSplinePoint` (`self.Zipline`) _index "Local"))
    (bind (_location_2 _tangent_2) (`SplineComponent.GetLocationAndTangentAtSplinePoint` (`self.Zipline`) (+ _index 1) "Local"))
    (`SplineMeshComponent.SetStartAndEnd` _returnvalue_2 _location _tangent _location_2 _tangent_2 true)
    (`StaticMeshComponent.SetStaticMesh` (`self.Mesh_1`) _mesh)
    (`StaticMeshComponent.SetStaticMesh` (`self.Mesh_2`) _mesh)))