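; Destructible target that drops a key pickup when its health is depleted.
; Damage updates health; at zero it applies a small radial damage, then once enables Destructible physics, spawns a physics-driven BP_KeyPickUp and later destroys itself.
; Box overlap turns on physics for kunai projectiles, then after a delay destroys the first kunai type, or the target itself for the second.
; A health bar widget linked to the target shows only while the player character is inside the Sphere.
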(event `self.ReceiveAnyDamage`
  (params (Damage :type "Float (single-precision)") (DamageType :type "DamageType Object Reference") (InstigatedBy :type "Controller Object Reference") (DamageCauser :type "Actor Object Reference"))
  (bind _returnvalue (`self.K2_GetActorLocation`))
  (bind _output_get (set `self.CurrentHealth` (- (`self.CurrentHealth`) Damage)))
  (set `self.HealthPercentage` (/ _output_get (`self.MaxHealth`)))
  (if (<= _output_get 0.0)
    (`KismetSystemLibrary.Delay` 0.3)
    (`GameplayStatics.ApplyRadialDamage` :`BaseDamage` 1.0 :`Origin` _returnvalue :`DamageRadius` 1.0 :`DamageCauser` null :`InstigatedByController` null)
    (`/Engine/EditorBlueprintResources/StandardMacros.DoOnce` false
      (:`Completed`
        (`PrimitiveComponent.SetSimulatePhysics` (`self.Destructible`) true)
        (bind _returnvalue_2 (`|SpawnActorFromClass` "/Game/DoorAndKey/BP_KeyPickUp.BP_KeyPickUp_C" (`KismetMathLibrary.Conv_VectorToTransform` _returnvalue) "AlwaysSpawn" "OverrideRootScale" null null))
        (`self.SetActorEnableCollision` _returnvalue_2 true)
        (`PrimitiveComponent.SetSimulatePhysics` (`/Game/Interactables/BP_BaseInteractable.InteractableMesh` _returnvalue_2) true)
        (`KismetSystemLibrary.Delay` 3.0)
        (`self.K2_DestroyActor`)))))

(event `self.Box.OnComponentBeginOverlap`
  (params (OverlappedComponent :type "PrimitiveComponent Object Reference") (OtherActor :type "Actor Object Reference") (OtherComp :type "PrimitiveComponent Object Reference") (OtherBodyIndex :type Integer) (bFromSweep :type Boolean) (SweepResult :type "HitResult Structure (by ref)"))
  (`|ExecutionSequence`
    (:`then_0`
      (bind _asbp_kunai_projectile (cast `/Game/Interactables/Projectiles/BP_Kunai_Projectile` OtherActor))
      (`PrimitiveComponent.SetSimulatePhysics` (`/Game/Interactables/BP_BaseInteractable.InteractableMesh` _asbp_kunai_projectile) true)
      (`KismetSystemLibrary.Delay` 0.5)
      (`/Engine/EditorBlueprintResources/StandardMacros.IsValid` _asbp_kunai_projectile
        (:`Is Valid`
          (`self.K2_DestroyActor` _asbp_kunai_projectile))))
    (:`then_1`
      (bind _asbp_kunai_projectile_2 (cast `/Game/Interactables/Projectiles/BP_Kunai_Projectile_2` OtherActor))
      (`PrimitiveComponent.SetSimulatePhysics` (`/Game/Interactables/BP_BaseInteractable.InteractableMesh` _asbp_kunai_projectile_2) true)
      (`KismetSystemLibrary.Delay` 0.5)
      (`self.K2_DestroyActor`))))

(event `self.ReceiveBeginPlay`
  (bind _output_get (set `self.Widget` (`self.Widget`)))
  (`SceneComponent.SetHiddenInGame` _output_get true false)
  (bind _astarget_with_key_health_bar (cast `/Game/Level_Assets/Target/TargetWithKeyHealthBar` (`WidgetComponent.GetUserWidgetObject` (`self.Widget`))))
  (set `/Game/Level_Assets/Target/TargetWithKeyHealthBar.Enemy` self _astarget_with_key_health_bar)
  (set `self.CurrentHealth` (`self.MaxHealth`)))

(event `self.Sphere.OnComponentBeginOverlap`
  (params (OverlappedComponent :type "PrimitiveComponent Object Reference") (OtherActor :type "Actor Object Reference") (OtherComp :type "PrimitiveComponent Object Reference") (OtherBodyIndex :type Integer) (bFromSweep :type Boolean) (SweepResult :type "HitResult Structure (by ref)"))
  (cast `/Game/Characters/Player/CH_MyCharacter` OtherActor)
  (bind _output_get (set `self.Widget` (`self.Widget`)))
  (`SceneComponent.SetHiddenInGame` _output_get false false))

(event `self.Sphere.OnComponentEndOverlap`
  (params (OverlappedComponent :type "PrimitiveComponent Object Reference") (OtherActor :type "Actor Object Reference") (OtherComp :type "PrimitiveComponent Object Reference") (OtherBodyIndex :type Integer))
  (cast `/Game/Characters/Player/CH_MyCharacter` OtherActor)
  (bind _output_get (set `self.Widget` (`self.Widget`)))
  (`SceneComponent.SetHiddenInGame` _output_get true false))

(fn `UserConstructionScript`)