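; Character stand-in, apparently for scene capture, that displays equipped gear on its own skeletal mesh.
; On BeginPlay it passes itself to the player's CH_MyCharacter and exposes equip and unequip events.
; Equipping replaces the slot's actor with a collision-disabled spawn snapped to item-defined sockets, paired for arms and feet; unequipping destroys it.
; HasWeaponSheathed swaps primary and secondary weapon sockets; left hands also accept armor.
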(event `self.ReceiveBeginPlay`
  (bind _asch_my_character (cast `/Game/Characters/Player/CH_MyCharacter` (`GameplayStatics.GetPlayerCharacter` 0)))
  (message `/Game/Interactables/BPI_RecorderComm.PassReference` _asch_my_character self))

(event `/Game/Interactables/BPI_RecorderComm.EquipItem`
  (params (ItemInfo :type "/Game/Interactables/FItemInfo Structure"))
  (`self.AttachItem` ItemInfo))

(event `/Game/Interactables/BPI_RecorderComm.Unequipitem`
  (params (ItemInfo :type "/Game/Interactables/FItemInfo Structure"))
  (`self.UnattachItem` ItemInfo))

(fn `AttachItem`
  (params (ItemInfo :type "/Game/Interactables/FItemInfo Structure"))
  (bind ((`ItemClass_15_ECB7889F469337B1E71877B3DB6FBFB8` _itemclass) (`ItemSlot_21_E9D9E5674B5D5D76EEFC34B530F53D45` _itemslot)) (break `/Game/Interactables/FItemInfo` ItemInfo))
  (bind ((`ItemClass_15_ECB7889F469337B1E71877B3DB6FBFB8` _itemclass_2) (`ItemSlot_21_E9D9E5674B5D5D76EEFC34B530F53D45` _itemslot_2)) (break `/Game/Interactables/FItemInfo` ItemInfo))
  (if (`self.Has Weapon Sheathed`)
    (switch `/Game/Interactables/ESlotType` _itemslot
      (:`NewEnumerator1`
        (`/Engine/EditorBlueprintResources/StandardMacros.IsValid` (`self.HeadItem`)
          (:`Is Valid`
            (`self.K2_DestroyActor` (`self.HeadItem`)))
          (:`Is Not Valid`
            _))
        (bind _returnvalue (`|SpawnActorFromClass` _itemclass (`self.GetTransform`) "AlwaysSpawn" "OverrideRootScale" null null))
        (bind _output_get (set `self.HeadItem` _returnvalue))
        (bind _asbp_base_armor (cast `/Game/Interactables/Armor/BP_BaseArmor` _output_get))
        (`self.K2_AttachToComponent` _asbp_base_armor (`self.SkeletalMesh`) (`.MainAttachPoint_11_18124FFF458DE104520B649B7B0AA808` (break `/Game/Interactables/Armor/FArmorInfo` (`/Game/Interactables/Armor/BP_BaseArmor.ArmorInfo` _asbp_base_armor))) "SnapToTarget" "SnapToTarget" "SnapToTarget" true)
        (`self.SetActorEnableCollision` _asbp_base_armor false))
      (:`NewEnumerator2`
        (`/Engine/EditorBlueprintResources/StandardMacros.IsValid` (`self.TorsoItem`)
          (:`Is Valid`
            (`self.K2_DestroyActor` (`self.TorsoItem`)))
          (:`Is Not Valid`
            _))
        (bind _returnvalue_2 (`|SpawnActorFromClass` _itemclass (`self.GetTransform`) "AlwaysSpawn" "OverrideRootScale" null null))
        (bind _output_get_2 (set `self.TorsoItem` _returnvalue_2))
        (bind _asbp_base_armor_2 (cast `/Game/Interactables/Armor/BP_BaseArmor` _output_get_2))
        (`self.K2_AttachToComponent` _asbp_base_armor_2 (`self.SkeletalMesh`) (`.MainAttachPoint_11_18124FFF458DE104520B649B7B0AA808` (break `/Game/Interactables/Armor/FArmorInfo` (`/Game/Interactables/Armor/BP_BaseArmor.ArmorInfo` _asbp_base_armor_2))) "SnapToTarget" "SnapToTarget" "SnapToTarget" true)
        (`self.SetActorEnableCollision` _asbp_base_armor_2 false))
      (:`NewEnumerator3`
        (`/Engine/EditorBlueprintResources/StandardMacros.IsValid` (`self.RightArmItem`)
          (:`Is Valid`
            (`self.K2_DestroyActor` (`self.RightArmItem`)))
          (:`Is Not Valid`
            _))
        (bind _returnvalue_3 (`|SpawnActorFromClass` _itemclass (`self.GetTransform`) "AlwaysSpawn" "OverrideRootScale" null null))
        (bind _output_get_3 (set `self.RightArmItem` _returnvalue_3))
        (bind _asbp_base_armor_3 (cast `/Game/Interactables/Armor/BP_BaseArmor` _output_get_3))
        (`self.K2_AttachToComponent` _asbp_base_armor_3 (`self.SkeletalMesh`) (`.RightAttachPoint_12_5B306C2A4C3B86A024584BA95DB13F55` (break `/Game/Interactables/Armor/FArmorInfo` (`/Game/Interactables/Armor/BP_BaseArmor.ArmorInfo` _asbp_base_armor_3))) "SnapToTarget" "SnapToTarget" "SnapToTarget" true)
        (`self.SetActorEnableCollision` _asbp_base_armor_3 false)
        (`/Engine/EditorBlueprintResources/StandardMacros.IsValid` (`self.LeftArmItem`)
          (:`Is Valid`
            (`self.K2_DestroyActor` (`self.LeftArmItem`)))
          (:`Is Not Valid`
            _))
        (bind _returnvalue_4 (`|SpawnActorFromClass` _itemclass (`self.GetTransform`) "AlwaysSpawn" "OverrideRootScale" null null))
        (bind _output_get_4 (set `self.LeftArmItem` _returnvalue_4))
        (bind _asbp_base_armor_4 (cast `/Game/Interactables/Armor/BP_BaseArmor` _output_get_4))
        (`self.K2_AttachToComponent` _asbp_base_armor_4 (`self.SkeletalMesh`) (`.LeftAttachPoint_13_BABE92454CFB169E6AF784B627D8A7BA` (break `/Game/Interactables/Armor/FArmorInfo` (`/Game/Interactables/Armor/BP_BaseArmor.ArmorInfo` _asbp_base_armor_4))) "SnapToTarget" "SnapToTarget" "SnapToTarget" true)
        (`self.SetActorEnableCollision` _asbp_base_armor_4 false))
      (:`NewEnumerator4`
        (`/Engine/EditorBlueprintResources/StandardMacros.IsValid` (`self.LegsItem`)
          (:`Is Valid`
            (`self.K2_DestroyActor` (`self.LegsItem`)))
          (:`Is Not Valid`
            _))
        (bind _returnvalue_5 (`|SpawnActorFromClass` _itemclass (`self.GetTransform`) "AlwaysSpawn" "OverrideRootScale" null null))
        (bind _output_get_5 (set `self.LegsItem` _returnvalue_5))
        (bind _asbp_base_armor_5 (cast `/Game/Interactables/Armor/BP_BaseArmor` _output_get_5))
        (`self.K2_AttachToComponent` _asbp_base_armor_5 (`self.SkeletalMesh`) (`.MainAttachPoint_11_18124FFF458DE104520B649B7B0AA808` (break `/Game/Interactables/Armor/FArmorInfo` (`/Game/Interactables/Armor/BP_BaseArmor.ArmorInfo` _asbp_base_armor_5))) "SnapToTarget" "SnapToTarget" "SnapToTarget" true)
        (`self.SetActorEnableCollision` _asbp_base_armor_5 false))
      (:`NewEnumerator5`
        (`/Engine/EditorBlueprintResources/StandardMacros.IsValid` (`self.RightFootItem`)
          (:`Is Valid`
            (`self.K2_DestroyActor` (`self.RightFootItem`)))
          (:`Is Not Valid`
            _))
        (bind _returnvalue_6 (`|SpawnActorFromClass` _itemclass (`self.GetTransform`) "AlwaysSpawn" "OverrideRootScale" null null))
        (bind _output_get_6 (set `self.RightFootItem` _returnvalue_6))
        (bind _asbp_base_armor_6 (cast `/Game/Interactables/Armor/BP_BaseArmor` _output_get_6))
        (`self.K2_AttachToComponent` _asbp_base_armor_6 (`self.SkeletalMesh`) (`.RightAttachPoint_12_5B306C2A4C3B86A024584BA95DB13F55` (break `/Game/Interactables/Armor/FArmorInfo` (`/Game/Interactables/Armor/BP_BaseArmor.ArmorInfo` _asbp_base_armor_6))) "SnapToTarget" "SnapToTarget" "SnapToTarget" true)
        (`self.SetActorEnableCollision` _asbp_base_armor_6 false)
        (`/Engine/EditorBlueprintResources/StandardMacros.IsValid` (`self.LeftFootItem`)
          (:`Is Valid`
            (`self.K2_DestroyActor` (`self.LeftFootItem`)))
          (:`Is Not Valid`
            _))
        (bind _returnvalue_7 (`|SpawnActorFromClass` _itemclass (`self.GetTransform`) "AlwaysSpawn" "OverrideRootScale" null null))
        (bind _output_get_7 (set `self.LeftFootItem` _returnvalue_7))
        (bind _asbp_base_armor_7 (cast `/Game/Interactables/Armor/BP_BaseArmor` _output_get_7))
        (`self.K2_AttachToComponent` _asbp_base_armor_7 (`self.SkeletalMesh`) (`.LeftAttachPoint_13_BABE92454CFB169E6AF784B627D8A7BA` (break `/Game/Interactables/Armor/FArmorInfo` (`/Game/Interactables/Armor/BP_BaseArmor.ArmorInfo` _asbp_base_armor_7))) "SnapToTarget" "SnapToTarget" "SnapToTarget" true)
        (`self.SetActorEnableCollision` _asbp_base_armor_7 false))
      (:`NewEnumerator6`
        (`/Engine/EditorBlueprintResources/StandardMacros.IsValid` (`self.PrimaryRightHandItem`)
          (:`Is Valid`
            (`self.K2_DestroyActor` (`self.PrimaryRightHandItem`)))
          (:`Is Not Valid`
            _))
        (bind _returnvalue_8 (`|SpawnActorFromClass` _itemclass (`self.GetTransform`) "AlwaysSpawn" "OverrideRootScale" null null))
        (bind _output_get_8 (set `self.PrimaryRightHandItem` _returnvalue_8))
        (bind _asbp_base_weapon (cast `/Game/Interactables/Weapons/BP_BaseWeapon` _output_get_8))
        (`self.K2_AttachToComponent` _asbp_base_weapon (`self.SkeletalMesh`) (`.SecondaryRightHand_16_0F2C71C8462FDE10961538A1F3C552FA` (break `/Game/Interactables/Weapons/FWeaponInfo` (`/Game/Interactables/Weapons/BP_BaseWeapon.WeaponInfo` _asbp_base_weapon))) "SnapToTarget" "SnapToTarget" "SnapToTarget" true)
        (`self.SetActorEnableCollision` _asbp_base_weapon false))
      (:`NewEnumerator7`
        (`/Engine/EditorBlueprintResources/StandardMacros.IsValid` (`self.PrimaryLeftHandItem`)
          (:`Is Valid`
            (`self.K2_DestroyActor` (`self.PrimaryLeftHandItem`)))
          (:`Is Not Valid`
            _))
        (bind _returnvalue_9 (`|SpawnActorFromClass` _itemclass (`self.GetTransform`) "AlwaysSpawn" "OverrideRootScale" null null))
        (bind _output_get_9 (set `self.PrimaryLeftHandItem` _returnvalue_9))
        (bind _asbp_base_weapon_2 (cast `/Game/Interactables/Weapons/BP_BaseWeapon` _output_get_9)
          (:`then`
            (`self.K2_AttachToComponent` _asbp_base_weapon_2 (`self.SkeletalMesh`) (`.SecondaryLeftHand_18_6D7A01794CA7BA5A188638B020EE3582` (break `/Game/Interactables/Weapons/FWeaponInfo` (`/Game/Interactables/Weapons/BP_BaseWeapon.WeaponInfo` _asbp_base_weapon_2))) "SnapToTarget" "SnapToTarget" "SnapToTarget" true)
            (`self.SetActorEnableCollision` _asbp_base_weapon_2 false))
          (:`CastFailed`
            (bind _asbp_base_armor_8 (cast `/Game/Interactables/Armor/BP_BaseArmor` _output_get_9))
            (`self.K2_AttachToComponent` _asbp_base_armor_8 (`self.SkeletalMesh`) (`.MainAttachPoint_11_18124FFF458DE104520B649B7B0AA808` (break `/Game/Interactables/Armor/FArmorInfo` (`/Game/Interactables/Armor/BP_BaseArmor.ArmorInfo` _asbp_base_armor_8))) "SnapToTarget" "SnapToTarget" "SnapToTarget" true)
            (`self.SetActorEnableCollision` _asbp_base_armor_8 false))))
      (:`NewEnumerator8`
        (`/Engine/EditorBlueprintResources/StandardMacros.IsValid` (`self.SecondaryRightHandItem`)
          (:`Is Valid`
            (`self.K2_DestroyActor` (`self.SecondaryRightHandItem`)))
          (:`Is Not Valid`
            _))
        (bind _returnvalue_10 (`|SpawnActorFromClass` _itemclass (`self.GetTransform`) "AlwaysSpawn" "OverrideRootScale" null null))
        (bind _output_get_10 (set `self.SecondaryRightHandItem` _returnvalue_10))
        (bind _asbp_base_weapon_3 (cast `/Game/Interactables/Weapons/BP_BaseWeapon` _output_get_10))
        (`self.K2_AttachToComponent` _asbp_base_weapon_3 (`self.SkeletalMesh`) (`.PrimaryRightHand_12_C0BFE3D145E3C135EE256EA8E84CB4D3` (break `/Game/Interactables/Weapons/FWeaponInfo` (`/Game/Interactables/Weapons/BP_BaseWeapon.WeaponInfo` _asbp_base_weapon_3))) "SnapToTarget" "SnapToTarget" "SnapToTarget" true)
        (`self.SetActorEnableCollision` _asbp_base_weapon_3 false))
      (:`NewEnumerator9`
        (`/Engine/EditorBlueprintResources/StandardMacros.IsValid` (`self.SecondaryLeftHandItem`)
          (:`Is Valid`
            (`self.K2_DestroyActor` (`self.SecondaryLeftHandItem`)))
          (:`Is Not Valid`
            _))
        (bind _returnvalue_11 (`|SpawnActorFromClass` _itemclass (`self.GetTransform`) "AlwaysSpawn" "OverrideRootScale" null null))
        (bind _output_get_11 (set `self.SecondaryLeftHandItem` _returnvalue_11))
        (bind _asbp_base_weapon_4 (cast `/Game/Interactables/Weapons/BP_BaseWeapon` _output_get_11)
          (:`then`
            (`self.K2_AttachToComponent` _asbp_base_weapon_4 (`self.SkeletalMesh`) (`.PrimaryLeftHand_14_1108E4D64692BFB228127ABB9A1BEBCE` (break `/Game/Interactables/Weapons/FWeaponInfo` (`/Game/Interactables/Weapons/BP_BaseWeapon.WeaponInfo` _asbp_base_weapon_4))) "SnapToTarget" "SnapToTarget" "SnapToTarget" true)
            (`self.SetActorEnableCollision` _asbp_base_weapon_4 false))
          (:`CastFailed`
            (bind _asbp_base_armor_9 (cast `/Game/Interactables/Armor/BP_BaseArmor` _output_get_11))
            (`self.K2_AttachToComponent` _asbp_base_armor_9 (`self.SkeletalMesh`) (`.MainAttachPoint_11_18124FFF458DE104520B649B7B0AA808` (break `/Game/Interactables/Armor/FArmorInfo` (`/Game/Interactables/Armor/BP_BaseArmor.ArmorInfo` _asbp_base_armor_9))) "SnapToTarget" "SnapToTarget" "SnapToTarget" true)
            (`self.SetActorEnableCollision` _asbp_base_armor_9 false))))
      (:`NewEnumerator10`
        (`/Engine/EditorBlueprintResources/StandardMacros.IsValid` null
          (:`Is Valid`
            (`self.K2_DestroyActor` (`self.AmuletItem`)))
          (:`Is Not Valid`
            _))
        (bind _returnvalue_12 (`|SpawnActorFromClass` _itemclass (`self.GetTransform`) "AlwaysSpawn" "OverrideRootScale" null null))
        (bind _output_get_12 (set `self.AmuletItem` _returnvalue_12))
        (bind _asbp_base_armor_10 (cast `/Game/Interactables/Armor/BP_BaseArmor` _output_get_12))
        (`self.K2_AttachToComponent` _asbp_base_armor_10 (`self.SkeletalMesh`) (`.MainAttachPoint_11_18124FFF458DE104520B649B7B0AA808` (break `/Game/Interactables/Armor/FArmorInfo` (`/Game/Interactables/Armor/BP_BaseArmor.ArmorInfo` _asbp_base_armor_10))) "SnapToTarget" "SnapToTarget" "SnapToTarget" true)
        (`self.SetActorEnableCollision` _asbp_base_armor_10 false)))
    (else
      (switch `/Game/Interactables/ESlotType` _itemslot_2
        (:`NewEnumerator1`
          (`/Engine/EditorBlueprintResources/StandardMacros.IsValid` (`self.HeadItem`)
            (:`Is Valid`
              (`self.K2_DestroyActor` (`self.HeadItem`)))
            (:`Is Not Valid`
              _))
          (bind _returnvalue_13 (`|SpawnActorFromClass` _itemclass_2 (`self.GetTransform`) "AlwaysSpawn" "OverrideRootScale" null null))
          (bind _output_get_13 (set `self.HeadItem` _returnvalue_13))
          (bind _asbp_base_armor_11 (cast `/Game/Interactables/Armor/BP_BaseArmor` _output_get_13))
          (`self.K2_AttachToComponent` _asbp_base_armor_11 (`self.SkeletalMesh`) (`.MainAttachPoint_11_18124FFF458DE104520B649B7B0AA808` (break `/Game/Interactables/Armor/FArmorInfo` (`/Game/Interactables/Armor/BP_BaseArmor.ArmorInfo` _asbp_base_armor_11))) "SnapToTarget" "SnapToTarget" "SnapToTarget" true)
          (`self.SetActorEnableCollision` _asbp_base_armor_11 false))
        (:`NewEnumerator2`
          (`/Engine/EditorBlueprintResources/StandardMacros.IsValid` (`self.TorsoItem`)
            (:`Is Valid`
              (`self.K2_DestroyActor` (`self.TorsoItem`)))
            (:`Is Not Valid`
              _))
          (bind _returnvalue_14 (`|SpawnActorFromClass` _itemclass_2 (`self.GetTransform`) "AlwaysSpawn" "OverrideRootScale" null null))
          (bind _output_get_14 (set `self.TorsoItem` _returnvalue_14))
          (bind _asbp_base_armor_12 (cast `/Game/Interactables/Armor/BP_BaseArmor` _output_get_14))
          (`self.K2_AttachToComponent` _asbp_base_armor_12 (`self.SkeletalMesh`) (`.MainAttachPoint_11_18124FFF458DE104520B649B7B0AA808` (break `/Game/Interactables/Armor/FArmorInfo` (`/Game/Interactables/Armor/BP_BaseArmor.ArmorInfo` _asbp_base_armor_12))) "SnapToTarget" "SnapToTarget" "SnapToTarget" true)
          (`self.SetActorEnableCollision` _asbp_base_armor_12 false))
        (:`NewEnumerator3`
          (`/Engine/EditorBlueprintResources/StandardMacros.IsValid` (`self.RightArmItem`)
            (:`Is Valid`
              (`self.K2_DestroyActor` (`self.RightArmItem`)))
            (:`Is Not Valid`
              _))
          (bind _returnvalue_15 (`|SpawnActorFromClass` _itemclass_2 (`self.GetTransform`) "AlwaysSpawn" "OverrideRootScale" null null))
          (bind _output_get_15 (set `self.RightArmItem` _returnvalue_15))
          (bind _asbp_base_armor_13 (cast `/Game/Interactables/Armor/BP_BaseArmor` _output_get_15))
          (`self.K2_AttachToComponent` _asbp_base_armor_13 (`self.SkeletalMesh`) (`.RightAttachPoint_12_5B306C2A4C3B86A024584BA95DB13F55` (break `/Game/Interactables/Armor/FArmorInfo` (`/Game/Interactables/Armor/BP_BaseArmor.ArmorInfo` _asbp_base_armor_13))) "SnapToTarget" "SnapToTarget" "SnapToTarget" true)
          (`self.SetActorEnableCollision` _asbp_base_armor_13 false)
          (`/Engine/EditorBlueprintResources/StandardMacros.IsValid` (`self.LeftArmItem`)
            (:`Is Valid`
              (`self.K2_DestroyActor` (`self.LeftArmItem`)))
            (:`Is Not Valid`
              _))
          (bind _returnvalue_16 (`|SpawnActorFromClass` _itemclass_2 (`self.GetTransform`) "AlwaysSpawn" "OverrideRootScale" null null))
          (bind _output_get_16 (set `self.LeftArmItem` _returnvalue_16))
          (bind _asbp_base_armor_14 (cast `/Game/Interactables/Armor/BP_BaseArmor` _output_get_16))
          (`self.K2_AttachToComponent` _asbp_base_armor_14 (`self.SkeletalMesh`) (`.LeftAttachPoint_13_BABE92454CFB169E6AF784B627D8A7BA` (break `/Game/Interactables/Armor/FArmorInfo` (`/Game/Interactables/Armor/BP_BaseArmor.ArmorInfo` _asbp_base_armor_14))) "SnapToTarget" "SnapToTarget" "SnapToTarget" true)
          (`self.SetActorEnableCollision` _asbp_base_armor_14 false))
        (:`NewEnumerator4`
          (`/Engine/EditorBlueprintResources/StandardMacros.IsValid` (`self.LegsItem`)
            (:`Is Valid`
              (`self.K2_DestroyActor` (`self.LegsItem`)))
            (:`Is Not Valid`
              _))
          (bind _returnvalue_17 (`|SpawnActorFromClass` _itemclass_2 (`self.GetTransform`) "AlwaysSpawn" "OverrideRootScale" null null))
          (bind _output_get_17 (set `self.LegsItem` _returnvalue_17))
          (bind _asbp_base_armor_15 (cast `/Game/Interactables/Armor/BP_BaseArmor` _output_get_17))
          (`self.K2_AttachToComponent` _asbp_base_armor_15 (`self.SkeletalMesh`) (`.MainAttachPoint_11_18124FFF458DE104520B649B7B0AA808` (break `/Game/Interactables/Armor/FArmorInfo` (`/Game/Interactables/Armor/BP_BaseArmor.ArmorInfo` _asbp_base_armor_15))) "SnapToTarget" "SnapToTarget" "SnapToTarget" true)
          (`self.SetActorEnableCollision` _asbp_base_armor_15 false))
        (:`NewEnumerator5`
          (`/Engine/EditorBlueprintResources/StandardMacros.IsValid` (`self.RightFootItem`)
            (:`Is Valid`
              (`self.K2_DestroyActor` (`self.RightFootItem`)))
            (:`Is Not Valid`
              _))
          (bind _returnvalue_18 (`|SpawnActorFromClass` _itemclass_2 (`self.GetTransform`) "AlwaysSpawn" "OverrideRootScale" null null))
          (bind _output_get_18 (set `self.RightFootItem` _returnvalue_18))
          (bind _asbp_base_armor_16 (cast `/Game/Interactables/Armor/BP_BaseArmor` _output_get_18))
          (`self.K2_AttachToComponent` _asbp_base_armor_16 (`self.SkeletalMesh`) (`.RightAttachPoint_12_5B306C2A4C3B86A024584BA95DB13F55` (break `/Game/Interactables/Armor/FArmorInfo` (`/Game/Interactables/Armor/BP_BaseArmor.ArmorInfo` _asbp_base_armor_16))) "SnapToTarget" "SnapToTarget" "SnapToTarget" true)
          (`self.SetActorEnableCollision` _asbp_base_armor_16 false)
          (`/Engine/EditorBlueprintResources/StandardMacros.IsValid` (`self.LeftFootItem`)
            (:`Is Valid`
              (`self.K2_DestroyActor` (`self.LeftFootItem`)))
            (:`Is Not Valid`
              _))
          (bind _returnvalue_19 (`|SpawnActorFromClass` _itemclass_2 (`self.GetTransform`) "AlwaysSpawn" "OverrideRootScale" null null))
          (bind _output_get_19 (set `self.LeftFootItem` _returnvalue_19))
          (bind _asbp_base_armor_17 (cast `/Game/Interactables/Armor/BP_BaseArmor` _output_get_19))
          (`self.K2_AttachToComponent` _asbp_base_armor_17 (`self.SkeletalMesh`) (`.LeftAttachPoint_13_BABE92454CFB169E6AF784B627D8A7BA` (break `/Game/Interactables/Armor/FArmorInfo` (`/Game/Interactables/Armor/BP_BaseArmor.ArmorInfo` _asbp_base_armor_17))) "SnapToTarget" "SnapToTarget" "SnapToTarget" true)
          (`self.SetActorEnableCollision` _asbp_base_armor_17 false))
        (:`NewEnumerator6`
          (`/Engine/EditorBlueprintResources/StandardMacros.IsValid` (`self.PrimaryRightHandItem`)
            (:`Is Valid`
              (`self.K2_DestroyActor` (`self.PrimaryRightHandItem`)))
            (:`Is Not Valid`
              _))
          (bind _returnvalue_20 (`|SpawnActorFromClass` _itemclass_2 (`self.GetTransform`) "AlwaysSpawn" "OverrideRootScale" null null))
          (bind _output_get_20 (set `self.PrimaryRightHandItem` _returnvalue_20))
          (bind _asbp_base_weapon_5 (cast `/Game/Interactables/Weapons/BP_BaseWeapon` _output_get_20))
          (`self.K2_AttachToComponent` _asbp_base_weapon_5 (`self.SkeletalMesh`) (`.PrimaryRightHand_12_C0BFE3D145E3C135EE256EA8E84CB4D3` (break `/Game/Interactables/Weapons/FWeaponInfo` (`/Game/Interactables/Weapons/BP_BaseWeapon.WeaponInfo` _asbp_base_weapon_5))) "SnapToTarget" "SnapToTarget" "SnapToTarget" true)
          (`self.SetActorEnableCollision` _asbp_base_weapon_5 false))
        (:`NewEnumerator7`
          (`/Engine/EditorBlueprintResources/StandardMacros.IsValid` (`self.PrimaryLeftHandItem`)
            (:`Is Valid`
              (`self.K2_DestroyActor` (`self.PrimaryLeftHandItem`)))
            (:`Is Not Valid`
              _))
          (bind _returnvalue_21 (`|SpawnActorFromClass` _itemclass_2 (`self.GetTransform`) "AlwaysSpawn" "OverrideRootScale" null null))
          (bind _output_get_21 (set `self.PrimaryLeftHandItem` _returnvalue_21))
          (bind _asbp_base_weapon_6 (cast `/Game/Interactables/Weapons/BP_BaseWeapon` _output_get_21)
            (:`then`
              (`self.K2_AttachToComponent` _asbp_base_weapon_6 (`self.SkeletalMesh`) (`.PrimaryLeftHand_14_1108E4D64692BFB228127ABB9A1BEBCE` (break `/Game/Interactables/Weapons/FWeaponInfo` (`/Game/Interactables/Weapons/BP_BaseWeapon.WeaponInfo` _asbp_base_weapon_6))) "SnapToTarget" "SnapToTarget" "SnapToTarget" true)
              (`self.SetActorEnableCollision` _asbp_base_weapon_6 false))
            (:`CastFailed`
              (bind _asbp_base_armor_18 (cast `/Game/Interactables/Armor/BP_BaseArmor` _output_get_21))
              (`self.K2_AttachToComponent` _asbp_base_armor_18 (`self.SkeletalMesh`) (`.MainAttachPoint_11_18124FFF458DE104520B649B7B0AA808` (break `/Game/Interactables/Armor/FArmorInfo` (`/Game/Interactables/Armor/BP_BaseArmor.ArmorInfo` _asbp_base_armor_18))) "SnapToTarget" "SnapToTarget" "SnapToTarget" true)
              (`self.SetActorEnableCollision` _asbp_base_armor_18 false))))
        (:`NewEnumerator8`
          (`/Engine/EditorBlueprintResources/StandardMacros.IsValid` (`self.SecondaryRightHandItem`)
            (:`Is Valid`
              (`self.K2_DestroyActor` (`self.SecondaryRightHandItem`)))
            (:`Is Not Valid`
              _))
          (bind _returnvalue_22 (`|SpawnActorFromClass` _itemclass_2 (`self.GetTransform`) "AlwaysSpawn" "OverrideRootScale" null null))
          (bind _output_get_22 (set `self.SecondaryRightHandItem` _returnvalue_22))
          (bind _asbp_base_weapon_7 (cast `/Game/Interactables/Weapons/BP_BaseWeapon` _output_get_22))
          (`self.K2_AttachToComponent` _asbp_base_weapon_7 (`self.SkeletalMesh`) (`.SecondaryRightHand_16_0F2C71C8462FDE10961538A1F3C552FA` (break `/Game/Interactables/Weapons/FWeaponInfo` (`/Game/Interactables/Weapons/BP_BaseWeapon.WeaponInfo` _asbp_base_weapon_7))) "SnapToTarget" "SnapToTarget" "SnapToTarget" true)
          (`self.SetActorEnableCollision` _asbp_base_weapon_7 false))
        (:`NewEnumerator9`
          (`/Engine/EditorBlueprintResources/StandardMacros.IsValid` (`self.SecondaryLeftHandItem`)
            (:`Is Valid`
              (`self.K2_DestroyActor` (`self.SecondaryLeftHandItem`)))
            (:`Is Not Valid`
              _))
          (bind _returnvalue_23 (`|SpawnActorFromClass` _itemclass_2 (`self.GetTransform`) "AlwaysSpawn" "OverrideRootScale" null null))
          (bind _output_get_23 (set `self.SecondaryLeftHandItem` _returnvalue_23))
          (bind _asbp_base_weapon_8 (cast `/Game/Interactables/Weapons/BP_BaseWeapon` _output_get_23)
            (:`then`
              (`self.K2_AttachToComponent` _asbp_base_weapon_8 (`self.SkeletalMesh`) (`.SecondaryLeftHand_18_6D7A01794CA7BA5A188638B020EE3582` (break `/Game/Interactables/Weapons/FWeaponInfo` (`/Game/Interactables/Weapons/BP_BaseWeapon.WeaponInfo` _asbp_base_weapon_8))) "SnapToTarget" "SnapToTarget" "SnapToTarget" true)
              (`self.SetActorEnableCollision` _asbp_base_weapon_8 false))
            (:`CastFailed`
              (bind _asbp_base_armor_19 (cast `/Game/Interactables/Armor/BP_BaseArmor` _output_get_23))
              (`self.K2_AttachToComponent` _asbp_base_armor_19 (`self.SkeletalMesh`) (`.MainAttachPoint_11_18124FFF458DE104520B649B7B0AA808` (break `/Game/Interactables/Armor/FArmorInfo` (`/Game/Interactables/Armor/BP_BaseArmor.ArmorInfo` _asbp_base_armor_19))) "SnapToTarget" "SnapToTarget" "SnapToTarget" true)
              (`self.SetActorEnableCollision` _asbp_base_armor_19 false))))
        (:`NewEnumerator10`
          (`/Engine/EditorBlueprintResources/StandardMacros.IsValid` (`self.AmuletItem`)
            (:`Is Valid`
              (`self.K2_DestroyActor` (`self.AmuletItem`)))
            (:`Is Not Valid`
              _))
          (bind _returnvalue_24 (`|SpawnActorFromClass` _itemclass_2 (`self.GetTransform`) "AlwaysSpawn" "OverrideRootScale" null null))
          (bind _output_get_24 (set `self.AmuletItem` _returnvalue_24))
          (bind _asbp_base_armor_20 (cast `/Game/Interactables/Armor/BP_BaseArmor` _output_get_24))
          (`self.K2_AttachToComponent` _asbp_base_armor_20 (`self.SkeletalMesh`) (`.MainAttachPoint_11_18124FFF458DE104520B649B7B0AA808` (break `/Game/Interactables/Armor/FArmorInfo` (`/Game/Interactables/Armor/BP_BaseArmor.ArmorInfo` _asbp_base_armor_20))) "SnapToTarget" "SnapToTarget" "SnapToTarget" true)
          (`self.SetActorEnableCollision` _asbp_base_armor_20 false))))))

(fn `UnattachItem`
  (params (ItemInfo :type "/Game/Interactables/FItemInfo Structure"))
  (switch `/Game/Interactables/ESlotType` (`.ItemSlot_21_E9D9E5674B5D5D76EEFC34B530F53D45` (break `/Game/Interactables/FItemInfo` ItemInfo))
    (:`NewEnumerator1`
      (`self.K2_DestroyActor` (`self.HeadItem`)))
    (:`NewEnumerator2`
      (`self.K2_DestroyActor` (`self.TorsoItem`)))
    (:`NewEnumerator3`
      (`self.K2_DestroyActor` (`self.RightArmItem`))
      (`self.K2_DestroyActor` (`self.LeftArmItem`)))
    (:`NewEnumerator4`
      (`self.K2_DestroyActor` (`self.LegsItem`)))
    (:`NewEnumerator5`
      (`self.K2_DestroyActor` (`self.RightFootItem`))
      (`self.K2_DestroyActor` (`self.LeftFootItem`)))
    (:`NewEnumerator6`
      (`self.K2_DestroyActor` (`self.PrimaryRightHandItem`)))
    (:`NewEnumerator7`
      (`self.K2_DestroyActor` (`self.PrimaryLeftHandItem`)))
    (:`NewEnumerator8`
      (`self.K2_DestroyActor` (`self.SecondaryRightHandItem`)))
    (:`NewEnumerator9`
      (`self.K2_DestroyActor` (`self.SecondaryLeftHandItem`)))
    (:`NewEnumerator10`
      (`self.K2_DestroyActor` (`self.AmuletItem`)))))

(fn `UserConstructionScript`)