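; BP_TargetWithKey is a damageable target that drops a key pickup when destroyed.
; AnyDamage subtracts damage from Health, and at zero or below the actor destroys itself and plays an explosion emitter and 2D sound.
; It then spawns a BP_KeyPickUp at its location, always spawning despite collision, with collision and mesh physics enabled on the pickup.
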(event `self.ReceiveAnyDamage`
  (params (Damage :type "Float (single-precision)") (DamageType :type "DamageType Object Reference") (InstigatedBy :type "Controller Object Reference") (DamageCauser :type "Actor Object Reference"))
  (bind _returnvalue (`self.K2_GetActorLocation`))
  (bind _output_get (set `self.Health` (- (`self.Health`) Damage)))
  (if (<= _output_get 0.0)
    (`self.K2_DestroyActor`)
    (`GameplayStatics.SpawnEmitterAtLocation` "/Game/StarterContent/Particles/P_Explosion.P_Explosion" _returnvalue)
    (`GameplayStatics.SpawnSound2D` "/Game/StarterContent/Audio/Explosion_Cue.Explosion_Cue" 1.0 1.0 0.0 null)
    (bind _returnvalue_2 (`|SpawnActorFromClass` "/Game/DoorAndKey/BP_KeyPickUp.BP_KeyPickUp_C" (`KismetMathLibrary.Conv_VectorToTransform` _returnvalue) "AlwaysSpawn" "OverrideRootScale" null null))
    (`self.SetActorEnableCollision` _returnvalue_2 true)
    (`PrimitiveComponent.SetSimulatePhysics` (`/Game/Interactables/BP_BaseInteractable.InteractableMesh` _returnvalue_2) true)))

(fn `UserConstructionScript`)